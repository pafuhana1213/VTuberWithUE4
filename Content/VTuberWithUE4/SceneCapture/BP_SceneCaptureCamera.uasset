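; BP_SceneCaptureCamera is a scene capture camera in VTuberWithUE4 that shows its render target on the VR spectator screen from BeginPlay.
; The construction script syncs the Camera and SceneCaptureComponent2D field of view to one variable and can restrict capture to a show-only actor list.
; A toggle weights the M_PostGreenBack post-process material on the capture, apparently for green-screen output.
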(event EventBeginPlay
  (Class|HeadMountedDisplayFunctionLibrary|SetSpectatorScreenMode "Texture")
  (Class|HeadMountedDisplayFunctionLibrary|SetSpectatorScreenTexture (Variables|/Script/Engine.SceneCaptureComponent2D|GetTextureTarget (Variables|Default|GetSceneCaptureComponent2D))))

(fn ConstructionScript
  (bind _scenecapturecomponent2d (Variables|Default|GetSceneCaptureComponent2D))
  (bind _showonlyactors (Variables|/Script/Engine.SceneCaptureComponent|GetShowOnlyActors _scenecapturecomponent2d))
  (Utilities|FlowControl|Sequence
    (:then_0
      ;[1 1 1] カメラのFOV(画角)調整
      (Variables|/Script/Engine.SceneCaptureComponent2D|SetFOVAngle (Variables|Default|GetSceneCaptureComponent2D) (Variables|Default|GetFov))
      (Camera|SetFieldOfView (Variables|Default|GetCamera) (Variables|Default|GetFov)))
    (:then_1
      ;[1 1 1] レンダーターゲットテクスチャに書き込むActorの制限
      (Variables|/Script/Engine.SceneCaptureComponent|SetPrimitiveRenderMode (Variables|Default|GetSceneCaptureComponent2D) (select (Variables|Default|GetUseShowOnlyList) "PRM_UseShowOnlyList" "PRM_RenderScenePrimitives"))
      (Utilities|Array|Clear _showonlyactors)
      (Utilities|Array|AppendArray _showonlyactors (Variables|Default|GetShowOnlyList)))
    (:then_2
      (Utilities|Struct|SetmembersinPostProcessSettings (Variables|/Script/Engine.SceneCaptureComponent2D|GetPostProcessSettings (Variables|Default|GetSceneCaptureComponent2D)) (Utilities|Struct|MakeWeightedBlendables (Utilities|Array|MakeArray (Utilities|Struct|MakeWeightedBlendable (select (Variables|Default|GetUseGreenBack) 1.0 0.0) "/Game/VTuberWithUE4/SceneCapture/M_PostGreenBack.M_PostGreenBack")))))))