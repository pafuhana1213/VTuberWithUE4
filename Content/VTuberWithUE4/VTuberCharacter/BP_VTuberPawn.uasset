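; VR pawn that drives a VTuber avatar from the HMD and motion controllers.
; Each Tick converts camera and controller transforms into mesh space as head and hand IK targets on AnimBP_VTuber, with axis remapping and an offset to stabilize FABRIK.
; Inputs set hand-pose rates on the AnimBP and facial morph targets on the mesh.
; It also resets VR tracking, adjusts origin height for Oculus, and toggles Sequence Recorder via console commands.
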(event Custom|UpdateCharacterIK
  (bind _camera (Variables|Default|GetCamera))
  (bind _relativerotation (Variables|/Script/Engine.SceneComponent|GetRelativeRotation _camera))
  ;[1 1 1] キャラクタのIK制御パラメータの更新
  ;;[1 0.2 0.2] 頭～腰の制御パラメータの更新
  (Variables|/Game/VTuberWithUE4/VTuberCharacter/Animations/AnimBP_VTuber.AnimBP_VTuber_C|SetHeadTransform (Variables|Default|GetAnimBP) (Math|Transform|MakeTransform (+ (Math|Transform|InverseTransformLocation (Transformation|GetWorldTransform (Variables|Default|GetCharacter)) (Transformation|GetWorldLocation (Variables|Default|GetCamera))) "0, 0,20.000000") (Math|Rotator|MakeRotator (* (.yaw _relativerotation) -1.0) (.roll _relativerotation) (* (.pitch _relativerotation) -1.0)) "1,1,1"))
  ;;[1 0.2 0.2] 左手の制御パラメータの更新
  ;; TODO：コントローラ毎のオフセット処理
  (Variables|/Game/VTuberWithUE4/VTuberCharacter/Animations/AnimBP_VTuber.AnimBP_VTuber_C|SetHandTransform_l (Variables|Default|GetAnimBP) (Math|Transform|ComposeTransforms (Transformation|GetWorldTransform (Variables|Default|GetMotionController_l)) (Math|Transform|InvertTransform (Transformation|GetWorldTransform (Variables|Default|GetCharacter)))))
  ;;[1 0.2 0.2] 右手の制御パラメータの更新
  ;; TODO：コントローラ毎のオフセット処理
  (Variables|/Game/VTuberWithUE4/VTuberCharacter/Animations/AnimBP_VTuber.AnimBP_VTuber_C|SetHandTransform_r (Variables|Default|GetAnimBP) (Math|Transform|ComposeTransforms (Transformation|GetWorldTransform (Variables|Default|GetMotionController_r)) (Math|Transform|InvertTransform (Transformation|GetWorldTransform (Variables|Default|GetCharacter))))))

(event EventTick
  (params (DeltaSeconds :type Float%20%28single-precision%29))
  (CallFunction|UpdateCharacterIK) ; キャラクタのIK制御パラメータの更新
)

(event EventBeginPlay
  (Utilities|FlowControl|Sequence
    (:then_0
      ;[1 1 1] VR関係の初期化
      (Class|HeadMountedDisplayFunctionLibrary|ResetOrientationandPosition 0.0 "OrientationAndPosition")
      (switch name (Class|HeadMountedDisplayFunctionLibrary|GetHMDDeviceName)
        (:OculusHMD
          (Transformation|AddLocalOffset (Variables|Default|GetVROrigin) (Math|Vector|MakeVector 0.0 0.0 (.z (Transformation|GetSocketLocation (Variables|Default|GetCharacter) "head"))) false false))))
    (:then_1
      ;[1 1 1] Tickで制御するAnimBPを保存 ( 参照関係が気になる方はBPインターフェイスで)
      (bind _asanim_bp_vtuber (Utilities|Casting|CastToAnimBP_VTuber (Components|SkeletalMesh|GetAnimInstance (Variables|Default|GetCharacter))))
      (Variables|Default|SetAnimBP _asanim_bp_vtuber))))

(event Input|ActionEvents|InputActionHandPeace_l
  (params (Key :type Key%20Structure))
  (bind _animbp (Variables|Default|GetAnimBP))
  ;[1 1 1] モーションコントローラ入力から、指のアニメーションに関するパラメータを制御
  ;;[1 0.2 0.2] チョキ
  (:Pressed
    (Variables|/Game/VTuberWithUE4/VTuberCharacter/Animations/AnimBP_VTuber.AnimBP_VTuber_C|SetHandPeaceRate_l _animbp 1.0))
  (:Released
    (Variables|/Game/VTuberWithUE4/VTuberCharacter/Animations/AnimBP_VTuber.AnimBP_VTuber_C|SetHandPeaceRate_l _animbp 0.0)))

(event Input|ActionEvents|InputActionHandPeace_r
  (params (Key :type Key%20Structure))
  (bind _animbp (Variables|Default|GetAnimBP))
  ;[1 1 1] モーションコントローラ入力から、指のアニメーションに関するパラメータを制御
  ;;[1 0.2 0.2] チョキ
  (:Pressed
    (Variables|/Game/VTuberWithUE4/VTuberCharacter/Animations/AnimBP_VTuber.AnimBP_VTuber_C|SetHandPeaceRate_r _animbp 1.0))
  (:Released
    (Variables|/Game/VTuberWithUE4/VTuberCharacter/Animations/AnimBP_VTuber.AnimBP_VTuber_C|SetHandPeaceRate_r _animbp 0.0)))

(event Input|ActionEvents|InputActionHandPointing_l
  (params (Key :type Key%20Structure))
  (bind _animbp (Variables|Default|GetAnimBP))
  ;[1 1 1] モーションコントローラ入力から、指のアニメーションに関するパラメータを制御
  ;;[1 0.2 0.2] 指差し
  (:Pressed
    (Variables|/Game/VTuberWithUE4/VTuberCharacter/Animations/AnimBP_VTuber.AnimBP_VTuber_C|SetHandPointingRate_l _animbp 1.0))
  (:Released
    (Variables|/Game/VTuberWithUE4/VTuberCharacter/Animations/AnimBP_VTuber.AnimBP_VTuber_C|SetHandPointingRate_l _animbp 0.0)))

(event Input|ActionEvents|InputActionHandPointing_r
  (params (Key :type Key%20Structure))
  (bind _animbp (Variables|Default|GetAnimBP))
  ;[1 1 1] モーションコントローラ入力から、指のアニメーションに関するパラメータを制御
  ;;[1 0.2 0.2] 指差し
  (:Pressed
    (Variables|/Game/VTuberWithUE4/VTuberCharacter/Animations/AnimBP_VTuber.AnimBP_VTuber_C|SetHandPointingRate_r _animbp 1.0))
  (:Released
    (Variables|/Game/VTuberWithUE4/VTuberCharacter/Animations/AnimBP_VTuber.AnimBP_VTuber_C|SetHandPointingRate_r _animbp 0.0)))

(event Input|ActionEvents|InputActionResetVR
  (params (Key :type Key%20Structure))
  ;[1 1 1] キャリブレーション処理
  (:Pressed
    (Class|HeadMountedDisplayFunctionLibrary|ResetOrientationandPosition 0.0 "OrientationAndPosition")))

(event Input|ActionEvents|InputActionRecord
  (params (Key :type Key%20Structure))
  ;[1 1 1] シーケンスレコーダーによる録画開始・停止
  (:Pressed
    (Utilities|FlowControl|FlipFlop
      (:A
        (Development|ExecuteConsoleCommand (Utilities|String|ToString(Text) (Utilities|Text|FormatText "RecordSequence {Class Name} {Actor Name}" (Utilities|Text|MakeLiteralText "Actor") (Utilities|Text|MakeLiteralText "BP_VTuberPawn"))) 0))
      (:B
        (Development|ExecuteConsoleCommand "StopRecordingSequence" 0)))))

(event Input|AxisEvents|InputAxisFaceChange_Down
  (params (AxisValue :type Float%20%28single-precision%29))
  ;[1 1 1] 左スティック押し込み+傾きによる表情切り替え
  (Components|SkeletalMesh|SetMorphTarget (Variables|Default|GetCharacter) (Utilities|Array|Get(acopy) (Variables|Default|GetFaceChangeMorphTagetNames) 2) AxisValue true))

(event Input|AxisEvents|InputAxisFaceChange_Up
  (params (AxisValue :type Float%20%28single-precision%29))
  ;[1 1 1] 左スティック押し込み+傾きによる表情切り替え
  (Components|SkeletalMesh|SetMorphTarget (Variables|Default|GetCharacter) (Utilities|Array|Get(acopy) (Variables|Default|GetFaceChangeMorphTagetNames)) AxisValue true))

(event Input|AxisEvents|InputAxisHandHold_l
  (params (AxisValue :type Float%20%28single-precision%29))
  ;[1 1 1] モーションコントローラ入力から、指のアニメーションに関するパラメータを制御
  ;;[1 0.2 0.2] グー
  (Variables|/Game/VTuberWithUE4/VTuberCharacter/Animations/AnimBP_VTuber.AnimBP_VTuber_C|SetHandHoldRate_l (Variables|Default|GetAnimBP) AxisValue))

(event Input|AxisEvents|InputAxisHandHold_r
  (params (AxisValue :type Float%20%28single-precision%29))
  ;[1 1 1] モーションコントローラ入力から、指のアニメーションに関するパラメータを制御
  ;;[1 0.2 0.2] グー
  (Variables|/Game/VTuberWithUE4/VTuberCharacter/Animations/AnimBP_VTuber.AnimBP_VTuber_C|SetHandHoldRate_r (Variables|Default|GetAnimBP) AxisValue))

(event Input|AxisEvents|InputAxisFaceChange_Right
  (params (AxisValue :type Float%20%28single-precision%29))
  ;[1 1 1] 左スティック押し込み+傾きによる表情切り替え
  (Components|SkeletalMesh|SetMorphTarget (Variables|Default|GetCharacter) (Utilities|Array|Get(acopy) (Variables|Default|GetFaceChangeMorphTagetNames) 1) AxisValue true))

(event Input|AxisEvents|InputAxisFaceChange_Left
  (params (AxisValue :type Float%20%28single-precision%29))
  ;[1 1 1] 左スティック押し込み+傾きによる表情切り替え
  (Components|SkeletalMesh|SetMorphTarget (Variables|Default|GetCharacter) (Utilities|Array|Get(acopy) (Variables|Default|GetFaceChangeMorphTagetNames) 3) AxisValue true))

(fn ConstructionScript)